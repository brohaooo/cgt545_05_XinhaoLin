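; BP_BNY is a multi-part character actor that feeds head orientation to its materials, likely for NPR shading.
; Construction makes lash, morph, hair, outline and lash overlay meshes follow the main skeletal mesh's pose, then sets up dynamic materials on all but the outline.
; GetHeadVector derives forward and right directions from head sockets.
; Tick pushes these into HeadForward and HeadRight parameters on main, lash, morph and hair meshes only.
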(event EventBeginPlay)

(event Collision|EventActorBeginOverlap
  (params (OtherActor :type Actor%20Object%20Reference)))

(event EventTick
  (params (DeltaSeconds :type Float%20%28single-precision%29))
  (CallFunction|UpdateMaterials (Variables|Default|GetSkeletalMesh))
  (CallFunction|UpdateMaterials (Variables|Default|GetLashMesh))
  (CallFunction|UpdateMaterials (Variables|Default|GetMorphMesh))
  (CallFunction|UpdateMaterials (Variables|Default|GetHairMesh)))

(fn ConstructionScript
  (bind _skeletalmesh (Variables|Default|GetSkeletalMesh))
  (Components|SkinnedMesh|SetLeaderPoseComponent (Variables|Default|GetLashMesh) _skeletalmesh true true)
  (Components|SkinnedMesh|SetLeaderPoseComponent (Variables|Default|GetMorphMesh) _skeletalmesh true true)
  (Components|SkinnedMesh|SetLeaderPoseComponent (Variables|Default|GetHairMesh) _skeletalmesh true true)
  (Components|SkinnedMesh|SetLeaderPoseComponent (Variables|Default|GetOutlineMesh) _skeletalmesh true true)
  (Components|SkinnedMesh|SetLeaderPoseComponent (Variables|Default|GetLashOverlayMesh) _skeletalmesh true true)
  (CallFunction|ConstructMaterials (Variables|Default|GetSkeletalMesh))
  (CallFunction|ConstructMaterials (Variables|Default|GetLashMesh))
  (CallFunction|ConstructMaterials (Variables|Default|GetMorphMesh))
  (CallFunction|ConstructMaterials (Variables|Default|GetHairMesh))
  (CallFunction|ConstructMaterials (Variables|Default|GetLashOverlayMesh)))

(fn ConstructMaterials
  (params (SkeletalMesh :type Skeletal%20Mesh%20Component%20Object%20Reference))
  (bind (_headforward _headright) (Utilities|GetHeadVector))
  (for (_array_element _array_index) (Rendering|Material|GetMaterials SkeletalMesh)
    (bind _asmaterial_instance_dynamic (Utilities|Casting|CastToMaterialInstanceDynamic _array_element)
      (:then
        (Rendering|Material|SetVectorParameterValue _asmaterial_instance_dynamic "HeadForward" _headforward :!class /Script/Engine.MaterialInstanceDynamic)
        (Rendering|Material|SetVectorParameterValue _asmaterial_instance_dynamic "HeadRight" _headright :!class /Script/Engine.MaterialInstanceDynamic))
      (:CastFailed
        (bind _returnvalue (Rendering|Material|CreateDynamicMaterialInstance SkeletalMesh _array_index _array_element "None" :!class /Script/Engine.PrimitiveComponent))
        (Rendering|Material|SetVectorParameterValue _returnvalue "HeadForward" _headforward :!class /Script/Engine.MaterialInstanceDynamic)
        (Rendering|Material|SetVectorParameterValue _returnvalue "HeadRight" _headright :!class /Script/Engine.MaterialInstanceDynamic))))
  (return 0))

(fn UpdateMaterials
  (params (SkeletalMesh :type Skeletal%20Mesh%20Component%20Object%20Reference))
  (bind (_headforward _headright) (Utilities|GetHeadVector))
  (Rendering|Material|SetVectorParameterValueonMaterials SkeletalMesh "HeadForward" (Math|Conversions|ToVector(LinearColor) _headforward))
  (Rendering|Material|SetVectorParameterValueonMaterials SkeletalMesh "HeadRight" (Math|Conversions|ToVector(LinearColor) _headright))
  (return))